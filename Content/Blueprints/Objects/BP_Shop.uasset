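; BP_Shop is an interactable shop actor that opens the shop UI.
; On Interact it calls the parent handler, creates a WBP_Shop widget with itself as OwnerShop, and adds it to the viewport.
; BeginPlay, overlap and Tick are disabled stubs, and the construction script only calls its parent.
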(event EventBeginPlay
  (|CallParentFunction) ; This node is disabled and will not be called.\nDrag off pins to build functionality.
)

(event Collision|EventActorBeginOverlap
  (params (OtherActor :type Actor%20Object%20Reference))
  (|CallParentFunction OtherActor) ; This node is disabled and will not be called.\nDrag off pins to build functionality.
)

(event EventTick
  (params (DeltaSeconds :type Float%20%28single-precision%29))
  (|CallParentFunction DeltaSeconds) ; This node is disabled and will not be called.\nDrag off pins to build functionality.
)

(event EventInteract
  (params (InstigatorPawn :type Player%20Character%20Object%20Reference))
  (|CallParentFunction InstigatorPawn)
  (bind _returnvalue (UserInterface|CreateWidget "/Game/Widgets/ShopWidgets/WBP_Shop.WBP_Shop_C" 0 self))
  (UserInterface|Viewport|AddtoViewport _returnvalue 0))

(fn ConstructionScript
  (|CallParentFunction))
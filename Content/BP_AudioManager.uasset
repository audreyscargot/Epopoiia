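; BP_AudioManager switches the music between a day and a night sound.
; An update-music dispatcher drives the switch with an IsDay flag, fading the audio component out, swapping the sound after a one-second delay, then fading back in.
; On BeginPlay it binds to that dispatcher and switches to night music only if the system clock reads earlier than 19:00.
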(event Custom|Update
  (params (isDay :type Boolean))
  (if isDay
    (CallFunction|UpdateMusic true)
    (else
      (CallFunction|UpdateMusic false))))

(event Custom|UpdateMusic
  (params (isDay :type Boolean))
  (bind _audiomanager (Variables|Default|GetAudioManager))
  (Audio|Components|Audio|FadeOut _audiomanager 1.0 0.0 "Linear" :!class /Script/Engine.AudioComponent)
  (Utilities|FlowControl|Delay 1.0)
  (Audio|Components|Audio|SetSound _audiomanager (select isDay (Variables|Default|GetDaySound) (Variables|Default|GetNightSound)))
  (Audio|Components|Audio|FadeIn _audiomanager 1.0 1.0 0.0 "Linear" :!class /Script/Engine.AudioComponent))

(event EventBeginPlay
  (EventDispatchers|BindEventtoUpdateMusicDispatcher (delegate Custom|Update))
  (if (not (>= (.hour (Math|DateTime|Now)) 19.0))
    (CallFunction|UpdateMusic false)))

(fn ConstructionScript)
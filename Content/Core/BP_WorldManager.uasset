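; BP_WorldManager switches the temple between day and night by toggling a night light and crossfading the matching music.
; On BeginPlay it binds to the temple update dispatcher and checks the system clock, starting in night state from 19:00 onward and otherwise playing day music.
; State changes require a valid NightLight, and music changes fade out, swap the sound after a delay, then fade back in.
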(event Custom|UpdateMusic
  (params (isNight :type Boolean))
  (bind _audiomanager (Variables|Default|GetAudioManager))
  (Audio|Components|Audio|FadeOut _audiomanager 1.0 0.0 "Linear" :!class /Script/Engine.AudioComponent)
  (Utilities|FlowControl|Delay 1.0)
  (Audio|Components|Audio|SetSound _audiomanager (select isNight (Variables|Default|GetNightSound) (Variables|Default|GetDaySound)))
  (Audio|Components|Audio|FadeIn _audiomanager 1.0 1.0 0.0 "Linear" :!class /Script/Engine.AudioComponent))

(event EventUpdateTempleState
  (params (_isDay :type Boolean))
  (bind _nightlight (Variables|Default|GetNightLight))
  (Variables|Default|GetNightLight
    (:then
      (if _isDay
        (Default|TurnOff _nightlight)
        (CallFunction|UpdateMusic false)
        (else
          (Default|Turnon _nightlight)
          (CallFunction|UpdateMusic true))))
    (:else)))

(event EventBeginPlay
  (EventDispatchers|BindEventtoUpdateTempleDispatcher (delegate EventUpdateTempleState))
  (if (>= (.hour (Math|DateTime|Now)) 19.0)
    (Class|WorldManager|UpdateTempleState false)
    (else
      (CallFunction|UpdateMusic false))))

(fn ConstructionScript)
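; Game mode for Epopoiia that matches the in-game day and night cycle to the real-world clock at startup.
; On BeginPlay it finds the SunMoonDaySequenceActor and, if valid, caches it and runs MakeTime once.
; MakeTime sets that actor's time of day from Now, but divides minutes by 60 before converting to double, so integer division leaves only the hour.
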(event Custom|MakeTime
  (bind _returnvalue (Math|DateTime|Now))
  (Class|DaySequenceActor|SetTimeOfDay (Variables|Default|GetNightDaySystem) (Math|Conversions|ToFloat(Integer) (+ (.hour _returnvalue) (/ (.minute _returnvalue) 60)))))

(event EventBeginPlay
  (bind _returnvalue (Actor|GetActorOfClass "/Script/DaySequence.SunMoonDaySequenceActor"))
  (Utilities|IsValid _returnvalue
    (:Is%20Valid
      (Variables|Default|SetNightDaySystem _returnvalue)
      (CallFunction|MakeTime))))

(fn ConstructionScript)
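; Player Blueprint for Epopoiia, extending a parent class with camera transitions, smooth grid push/pull movement, inventory opening and vocabulary handoff to the game instance.
; SetCameraView blends camera boom transform and arm length on a Timeline, then creates the phone widget.
; A looping timer writes player location to a material parameter collection for occlusion.
; Temporary quit input and debug keys exercise inventory, grid, seed and reviews.
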(event Input|EnhancedActionEvents|EnhancedInputActionIA_TEMPQuit
  (params (ActionValue :type Boolean) (ElapsedSeconds :type Float%20%28double-precision%29) (TriggeredSeconds :type Float%20%28double-precision%29) (InputAction :type Input%20Action%20Object%20Reference :default "/Game/Input/IA_TEMPQuit.IA_TEMPQuit"))
  ;[0.15 0.15 0.15 0.5] TEMP : Quit Game TO BE MODIFIED
  (:Started
    (Game|QuitGame 0 "Quit" false)))

(event Input|EnhancedActionEvents|EnhancedInputActionIA_OpenInventory
  (params (ActionValue :type Boolean) (ElapsedSeconds :type Float%20%28double-precision%29) (TriggeredSeconds :type Float%20%28double-precision%29) (InputAction :type Input%20Action%20Object%20Reference :default "/Game/Input/GameInput/IA_OpenInventory.IA_OpenInventory"))
  (:Started
    (Utilities|IsValid (Variables|Default|GetInventoryWidget)
      (:Is%20Not%20Valid
        (bind _returnvalue (UserInterface|CreateWidget "/Game/Widgets/Inventory/WBP_Inventory.WBP_Inventory_C" (Game|GetPlayerController 0) self))
        (bind _output_get (Variables|Default|SetInventoryWidget _returnvalue))
        (UserInterface|Viewport|AddtoViewport _output_get 0)))))

(event EventSmoothGridMove
  (params (_basePosition :type Vector :default "0, 0, 0") (_displacement :type Vector :default "0, 0, 0") (_movementSpeed :type Float%20%28single-precision%29))
  ;[0.0242 0.09773 0.15 0.5] Push Pull smooth move
  (Components|Timeline|SetPlayRate (Variables|Default|GetSmoothMove) (/ 1.0 _movementSpeed))
  (bind _alpha (Timeline|SmoothMove PlayFromStart)
    (:Update
      (Transformation|SetActorLocation (Math|Vector|Lerp(Vector) _basePosition _displacement _alpha) false false)
      (Class|PlayerCharacter|CallDelegate _displacement false))))

(event EventBeginPlay
  (|CallParentFunction)
  (Utilities|Time|SetTimerbyFunctionName 0 "CheckForOcclusion" 0.01 true)
  (bind _asgi_main (Utilities|Casting|CastToGI_Main (Game|GetGameInstance)))
  (Variables|/Script/Epopoiia.GameInstanceMain|SetplayerVocabulary _asgi_main (Variables|/Script/Epopoiia.MythipediaManager|Getvocabulary (Variables|Default|GetMythipediaManager))))

(event EventSetCameraView
  (params (bIsPhoneView :type Boolean) (CameraTransform :type Transform) (ArmLength :type Float%20%28single-precision%29))
  (bind (_location _rotation _scale) (Math|Transform|BreakTransform CameraTransform))
  (bind _cameraboom (Variables|Default|GetCameraBoom))
  ;[0.5625 0.08285 0.533 0.5] CameraView change
  (|CallParentFunction bIsPhoneView CameraTransform ArmLength)
  (bind _phonewidget (Variables|Default|GetPhoneWidget)
    (:then
      (Class|DetectUserWidget|RemoveWidget _phonewidget))
    (:else
      _))
  (Variables|Default|SetTarget%20Arm%20Length%20Current (Variables|/Script/Engine.SpringArmComponent|GetTargetArmLength _cameraboom))
  (Variables|Default|SetCameraBoom%20Transform%20Current (Transformation|GetRelativeTransform _cameraboom))
  (Components|Timeline|SetPlayRate (Variables|Default|GetTimeline) 1.0)
  (bind _alpha (Timeline|Timeline PlayFromStart)
    (:Update
      (Transformation|SetRelativeTransform (Variables|Default|GetCameraBoom) (Math|Transform|Lerp(Transform) (Variables|Default|GetCameraBoom%20Transform%20Current) (select bIsPhoneView (Math|Transform|MakeTransform _location (Math|Transform|TransformRotation (Transformation|GetWorldTransform (Variables|Default|GetCapsuleComponent)) _rotation) _scale) CameraTransform) _alpha) false false)
      (Variables|/Script/Engine.SpringArmComponent|SetTargetArmLength (Variables|Default|GetCameraBoom) (Math|Float|Lerp (Variables|Default|GetTarget%20Arm%20Length%20Current) ArmLength _alpha)))
    (:Finished
      (Class|PlayerCharacter|CreatePhoneWidget "/Game/Widgets/PhoneWidgets/WBP_PhoneMain.WBP_PhoneMain_C"))))

(event Input|KeyboardEvents|DebugKeyJ
  (params (Key :type Key%20Structure :default "None") (ActionValue :type Input%20Action%20Value%20Structure))
  ;[1 0.01094 0 0.5] DEBUG
  (:Pressed
    (for _array_element (Variables|/Script/Epopoiia.InventoryComponent|GetInventory (Variables|Default|GetInventory))
      (Development|PrintString (Utilities|String|ToString(Integer) _array_element)))))

(event Input|KeyboardEvents|DebugKeyU
  (params (Key :type Key%20Structure :default "None") (ActionValue :type Input%20Action%20Value%20Structure))
  (bind _inventory (Variables|Default|GetInventory))
  ;[1 0.01094 0 0.5] DEBUG
  (:Pressed
    (Class|InventoryComponent|UseItem _inventory (Utilities|Array|Get(acopy) (Variables|/Script/Epopoiia.InventoryComponent|GetInventory _inventory)))))

(event Input|KeyboardEvents|DebugKeyY
  (params (Key :type Key%20Structure :default "None") (ActionValue :type Input%20Action%20Value%20Structure))
  ;[1 0.01094 0 0.5] DEBUG
  (:Pressed
    (bind _asepopoiia_game_mode (Utilities|Casting|CastToEpopoiiaGameMode (Game|GetGameMode)))
    (for _array_element (Variables|/Script/Epopoiia.EpopoiiaGameMode|GetGrid _asepopoiia_game_mode)
      (Development|PrintString (Utilities|String|ToString(Vector) _array_element)))))

(event Input|KeyboardEvents|DebugKeyR
  (params (Key :type Key%20Structure :default "None") (ActionValue :type Input%20Action%20Value%20Structure))
  (bind _reviewmanager (Variables|Default|GetReviewManager))
  (bind _reviews (Variables|/Script/Epopoiia.ReviewManagerComponent|Getreviews _reviewmanager))
  (bind _returnvalue (Utilities|Array|LastIndex _reviews))
  (bind _output (Utilities|Array|Get(acopy) _reviews _returnvalue))
  (bind (_reviewnpcname _reviewgrade _reviewtext) (Utilities|Struct|BreakReviewStruct _output))
  ;[1 0.01094 0 0.5] DEBUG
  (:Pressed
    (Class|ReviewManagerComponent|MakeReview _reviewmanager false)
    (Development|PrintString _reviewtext)
    (Development|PrintString (Utilities|String|ToString(Integer) _reviewgrade))))

(event Input|KeyboardEvents|DebugKeyC
  (params (Key :type Key%20Structure :default "None") (ActionValue :type Input%20Action%20Value%20Structure))
  ;[1 0.01094 0 0.5] DEBUG
  (:Pressed
    (Utilities|Array|Clear (Variables|/Script/Epopoiia.ReviewManagerComponent|Getreviews (Variables|Default|GetReviewManager)))
    (bind _asgi_main (Utilities|Casting|CastToGI_Main (Game|GetGameInstance)))
    (Variables|/Script/Epopoiia.GameInstanceMain|Setreviews _asgi_main (Variables|/Script/Epopoiia.ReviewManagerComponent|Getreviews (Variables|Default|GetReviewManager)))
    (Class|GameInstanceMain|SaveReviews _asgi_main)))

(event Input|KeyboardEvents|DebugKeyI
  (params (Key :type Key%20Structure :default "None") (ActionValue :type Input%20Action%20Value%20Structure))
  ;[1 0.01094 0 0.5] DEBUG
  (:Pressed
    (bind _asgi_main (Utilities|Casting|CastToGI_Main (Game|GetGameInstance)))
    (bind _output_get (Variables|/Script/Epopoiia.GameInstanceMain|Setseed _asgi_main (- (Variables|/Script/Epopoiia.GameInstanceMain|Getseed _asgi_main) 1)))
    (Development|PrintString (Utilities|String|ToString(Integer) _output_get))))

(fn ConstructionScript)

(fn CheckforOcclusion
  (Rendering|Material|SetVectorParameterValue "/Game/Art/Mat/Epopoiia_ParametersCollection.Epopoiia_ParametersCollection" "PlayerLocation" (Math|Conversions|ToLinearColor(Vector) (Transformation|GetActorLocation)) :!class /Script/Engine.KismetMaterialLibrary))
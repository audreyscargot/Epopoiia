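; BP_NightLight is a light that fades on and off through its TurnOn and TurnOff events.
; TurnOn activates two Niagara effects and plays a timeline that lerps the intensity of two point lights up from zero.
; TurnOff deactivates the effects and reverses the same timeline.
; At BeginPlay the timeline play rate is set to the inverse of the Time variable, so that variable controls fade duration.
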(event Custom|TurnOn
  (Components|Activation|Activate (Variables|Default|GetNiagara01) false)
  (bind _alpha (Timeline|ONTimeline Play)
    (:Update
      (Rendering|Components|Light|SetIntensity (Variables|Default|GetPL02) (Math|Float|Lerp 0.0 2.0 _alpha)))))

(event Custom|TurnOff
  (Components|Activation|Deactivate (Variables|Default|GetNiagara01))
  (bind _alpha (Timeline|ONTimeline Reverse)
    (:Update
      (Rendering|Components|Light|SetIntensity (Variables|Default|GetPL02) (Math|Float|Lerp 0.0 2.0 _alpha)))))

(event EventBeginPlay
  (Components|Timeline|SetPlayRate (Variables|Default|GetONTimeline) (/ 1.0 (Variables|Default|GetTime))))

(fn ConstructionScript)
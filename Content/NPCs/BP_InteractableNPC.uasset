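; Interactable NPC Blueprint that offers quest dialogue and shows a feedback widget while it has a current quest.
; InitFeedback sets widget visibility from the NPC's entry in GI_Main's QuestsOfDay, looked up by NpcID.
; Interact hides the widget, then uses QuestComponent's current quest to open WBP_DialogueWidget if DialogueWidgetRef is invalid.
; Opening dialogue also loops the talking animation and calls AddToPlayerVocabulary on the instigating pawn.
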(event EventInteract
  (params (InstigatorPawn :type Player%20Character%20Object%20Reference))
  (bind _questcomponent (Variables|Default|GetQuestComponent))
  (bind _npcquest (Variables|/Script/Epopoiia.QuestComponent|GetNPCquest _questcomponent))
  (|CallParentFunction InstigatorPawn)
  (CallFunction|SetQuestFeedbackVisibility false)
  (if (Utilities|Array|IsValidIndex (.quest _npcquest) (.currentquestindex _npcquest))
    (Utilities|IsValid (Variables|Default|GetDialogueWidget_ref)
      (:Is%20Not%20Valid
        (bind _returnvalue (UserInterface|CreateWidget "/Game/Widgets/DialogueWidget/WBP_DialogueWidget.WBP_DialogueWidget_C" 0 (.questdialogueindex (Utilities|Array|Get(acopy) (.questdialoguenpc _npcquest) (.currentquestindex _npcquest))) (Utilities|Array|Get(acopy) (.quest _npcquest) (.currentquestindex _npcquest)) self))
        (UserInterface|Viewport|AddtoViewport _returnvalue 0)
        (Components|Animation|PlayAnimation (Variables|Default|GetSkeletalMesh) "/Game/Art/NPC/AS_Talking.AS_Talking" true)
        (Class|InteractableNPC|AddtoPlayerVocabulary InstigatorPawn)))))

(event EventBeginPlay
  (|CallParentFunction))

(event EventInitFeedback
  (CallFunction|SetQuestFeedbackVisibility true))

(fn ConstructionScript)

(fn SetQuestFeedbackVisibility
  (params (shouldBeVisible :type Boolean))
  (bind _returnvalue (Game|GetGameInstance))
  (bind _widget (Variables|Default|GetWidget))
  (bind _npcid (Variables|Default|GetnpcID))
  (bind _asgi_main (Utilities|Casting|CastToGI_Main _returnvalue))
  (bind _questsofday (Variables|/Script/Epopoiia.GameInstanceMain|GetquestsOfDay _asgi_main))
  (bind _output (Utilities|Array|Get(acopy) _questsofday _npcid))
  (if shouldBeVisible
    (Rendering|SetVisibility _widget (Utilities|Array|IsValidIndex (.quest _output) (.currentquestindex _output)) false)
    (else
      (Rendering|SetVisibility _widget false false))))